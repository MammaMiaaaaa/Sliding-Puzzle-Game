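; BP_SlidingPuzzle is an actor that lays out a numbered sliding-puzzle board.
; The construction script spawns mesh and text components in a grid from SquareCount, SquareDivide and Spacing, labelling each from the Puzzle array.
; The zero entry is hidden as the empty slot, and the per-character text offset currently adds nothing.
; The event graph is empty, so no sliding logic exists here.
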(event `self.ReceiveBeginPlay`)

(fn `UserConstructionScript`
  (for _index (range (+ (`self.SquareCount`) 1))
    (bind _returnvalue (`KismetMathLibrary.Conv_IntToDouble` (* (mod _index (`self.SquareDivide`)) (`self.Spacing`))))
    (bind _returnvalue_2 (`KismetMathLibrary.Conv_IntToDouble` (* (/ _index (`self.SquareDivide`)) (* (`self.Spacing`) -1))))
    (bind _returnvalue_3 (`AddComponent|NODE_AddStaticMeshComponent-0` :`RelativeTransform` (`KismetMathLibrary.MakeTransform` (`KismetMathLibrary.MakeVector` _returnvalue 0.0 _returnvalue_2))))
    (`KismetArrayLibrary.Array_Add` (`self.BoxPuzzle`) _returnvalue_3)
    (set `self.TextBox` (`KismetTextLibrary.Conv_IntToText` (`|GetArrayItem` (`self.Puzzle`) _index)))
    (set `self.MinusDistanceX` 0)
    (for _ (range 1 (+ (`KismetStringLibrary.Len` (`KismetTextLibrary.Conv_TextToString` (`self.TextBox`))) 1))
      (bind _output_get (set `self.MinusDistanceX` (- (`self.MinusDistanceX`) 0))))
    (bind _returnvalue_4 (`AddComponent|NODE_AddTextRenderComponent-0` :`RelativeTransform` (`KismetMathLibrary.MakeTransform` (`KismetMathLibrary.MakeVector` (+ _returnvalue _output_get) (`self.DistanceTextY`) _returnvalue_2) (struct :`Yaw` 90.0) (2.0 2.0 2.0))))
    (`KismetArrayLibrary.Array_Add` (`self.TextPuzzle`) _returnvalue_4)
    (if (`KismetTextLibrary.EqualEqual_TextText` (`self.TextBox`) "0")
      (`SceneComponent.SetVisibility` (`|GetArrayItem` (`self.BoxPuzzle`) _index) false false)
      (`SceneComponent.SetVisibility` (`|GetArrayItem` (`self.TextPuzzle`) _index) false false)
      (else
        (`TextRenderComponent.K2_SetText` _returnvalue_4 (`self.TextBox`))))))