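; Player controller for a sliding number puzzle that shows the cursor and lets the player click tiles to move them.
; A left click traces under the cursor and finds the hit mesh's index in the puzzle actor's box array.
; If the left neighbour is the empty 0 in the same row, a timeline lerps both boxes and texts, swapping number and box entries on each update.
; Only leftward sliding is implemented.
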(event `self.ReceiveBeginPlay`
  (set `self.bShowMouseCursor` true)
  (bind _returnvalue (`GameplayStatics.GetActorOfClass` null))
  (set `self.BP_Puzzle` null _returnvalue)
  (set `self.Arr_TextPuzzle` (`/Game/PC_Control.TextPuzzle` (`.BP_Puzzle` (`self.BP_Puzzle`)))))

(event `Key|LeftMouseButton`
  (params (Key :type "Key Structure"))
  (bind _selected_index (`self.Selected_Index`))
  (bind _arr_box (`self.Arr_Box`))
  (bind _selected_index_2 (`self.Selected_Index`))
  (bind _arr_textpuzzle (`self.Arr_TextPuzzle`))
  (bind _selected_index_3 (`self.Selected_Index`))
  (bind _output (`|GetArrayItem` _arr_textpuzzle _selected_index))
  (bind _output_2 (`|GetArrayItem` _arr_box _selected_index))
  (bind _returnvalue (- _selected_index 1))
  (bind _returnvalue_2 (- _selected_index_2 1))
  (bind _boxpuzzle (`/Game/PC_Control.BoxPuzzle` (`.BP_Puzzle` (`self.BP_Puzzle`))))
  (bind _output_3 (`|GetArrayItem` _arr_textpuzzle _returnvalue))
  (bind _output_4 (`|GetArrayItem` _arr_box _returnvalue))
  (:`Pressed`
    (bind _asstatic_mesh_component (cast `StaticMeshComponent` (`.HitComponent` (`GameplayStatics.BreakHitResult` (`self.GetHitResultUnderCursorByChannel` (`GameplayStatics.GetPlayerController` 0) "TraceTypeQuery1" true)))))
    (set `self.Selected_Index` (`KismetArrayLibrary.Array_Find` _boxpuzzle _asstatic_mesh_component))
    (set `self.Arr_Box` _boxpuzzle)
    (set `self.Arr_Number` (`/Game/PC_Control.Puzzle` (`.BP_Puzzle` (`self.BP_Puzzle`))))
    (for _ (range 2)
      (if (`KismetMathLibrary.Conv_IntToBool` (`KismetMathLibrary.And_IntInt` (`KismetMathLibrary.Conv_BoolToInt` (== (`|GetArrayItem` (`self.Arr_Number`) (- (`self.Selected_Index`) 1)) 0)) (`KismetMathLibrary.Conv_BoolToInt` (== (`self.getRowColumn` _selected_index_3) (`self.getRowColumn` (- _selected_index_3 1))))))
        ;[1 1 1] geser kotak ke kiri
        (`KismetSystemLibrary.PrintString` (`KismetSystemLibrary.GetDisplayName` _output))
        (set `self.SourceText` (`SceneComponent.K2_GetComponentLocation` _output))
        (set `self.DestText` (`SceneComponent.K2_GetComponentLocation` _output_3))
        (set `self.SourceBox` (`SceneComponent.K2_GetComponentLocation` _output_2))
        (set `self.DestBox` (`SceneComponent.K2_GetComponentLocation` _output_4))
        (bind (_direction _newtrack_0) (`Timeline|Transform Box` :!via `PlayFromStart`)
          (:`Update`
            (`SceneComponent.K2_SetWorldLocation` _output_2 (`KismetMathLibrary.VLerp` (`self.SourceBox`) (`self.DestBox`) _newtrack_0) false false)
            (`SceneComponent.K2_SetWorldLocation` _output_4 (`KismetMathLibrary.VLerp` (`self.DestBox`) (`self.SourceBox`) _newtrack_0) false false)
            (`SceneComponent.K2_SetWorldLocation` _output (`KismetMathLibrary.VLerp` (`self.SourceText`) (`self.DestText`) _newtrack_0) false false)
            (`SceneComponent.K2_SetWorldLocation` _output_3 (`KismetMathLibrary.VLerp` (`self.DestText`) (`self.SourceText`) _newtrack_0) false false)
            ;[1 1 1] swap kiri
            (`KismetArrayLibrary.Array_Swap` (`self.Arr_Number`) _selected_index_2 _returnvalue_2)
            (`KismetArrayLibrary.Array_Swap` (`self.Arr_Box`) _selected_index_2 _returnvalue_2)))))))

(fn `getRowColumn`
  (params (Index :type Integer))
  (returns (Row :type Integer) (Column :type Integer))
  (bind _returnvalue (`KismetMathLibrary.Sqrt` (`KismetMathLibrary.Conv_IntToDouble` (`/Game/PC_Control.SquareCount` (`.BP_Puzzle` (`self.BP_Puzzle`))))))
  (return (/ Index _returnvalue) (mod Index (`KismetMathLibrary.FTrunc` _returnvalue))))

(fn `UserConstructionScript`)